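; BP_Interactable is an interactable actor that changes the mouse cursor on hover and detects double-clicks.
; On BeginPlay it binds its cursor-over and click events, switching the cursor between Hand and Default.
; A click flag cleared after a short delay turns a second click into a call to OnDoubleClicked, which is empty here.
; CheckDoubleClick repeats that logic without the delay and is not called in this file.
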(event `OnClickedDelegate` :!signature `self.OnClicked`
  (params (TouchedActor :type "Actor Object Reference") (ButtonPressed :type "Key Structure" :default "None"))
  (if (`self.IsClicking`)
    (`self.OnDoubleClicked`)
    (set `self.IsClicking` false)
    (else
      (set `self.IsClicking` true)
      (`KismetSystemLibrary.Delay` 0.4)
      (set `self.IsClicking` false))))

(event `OnBeginCursorOverDelegate` :!signature `self.OnBeginCursorOver`
  (params (TouchedActor :type "Actor Object Reference"))
  (set `PlayerController.CurrentMouseCursor` "Hand" (`GameplayStatics.GetPlayerController` 0)))

(event `self.ReceiveBeginPlay`
  (add `self.OnBeginCursorOver` (delegate `OnBeginCursorOverDelegate`))
  (add `self.OnEndCursorOver` (delegate `OnEndCursorOverDelegate`))
  (add `self.OnClicked` (delegate `OnClickedDelegate`)))

(event `OnEndCursorOverDelegate` :!signature `self.OnEndCursorOver`
  (params (TouchedActor :type "Actor Object Reference"))
  (set `PlayerController.CurrentMouseCursor` "Default" (`GameplayStatics.GetPlayerController` 0)))

(fn `CheckDoubleClick`
  (if (`self.IsClicking`)
    (`self.OnDoubleClicked`)
    (set `self.IsClicking` false)
    (else
      (set `self.IsClicking` true))))

(fn `OnDoubleClicked`)

(fn `UserConstructionScript`)
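; BP_Before is an event actor representing a "before" state that can be swapped for a linked After actor.
; Double-clicking it runs the parent handler, then reports itself as wrong to BP_EventManager, obtained by casting the game mode.
; Play shows the After actor with collision enabled, if valid, then hides this actor and disables its collision.
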(fn `OnDoubleClicked`
  (`parent.OnDoubleClicked`)
  (bind _asbp_event_manager (cast `/Game/Blueprints/Event/BP_EventManager` (`GameplayStatics.GetGameMode`)))
  (`/Game/Blueprints/Event/BP_EventManager.OnWrong` _asbp_event_manager self))

(fn `Play`
  (bind _after (`self.after`))
  (`/Engine/EditorBlueprintResources/StandardMacros.IsValid` _after
    (:`Is Valid`
      (`self.SetActorHiddenInGame` _after false)
      (`self.SetActorEnableCollision` _after true))
    (:`Is Not Valid`
      _))
  (`self.SetActorHiddenInGame` true)
  (`self.SetActorEnableCollision` false))

(fn `UserConstructionScript`)
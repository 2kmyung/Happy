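; BP_After is the "after" state of an event object, paired with a Before actor and reported as a right pick when double-clicked.
; Reset shows the Before actor with collision and hides this one without collision; the construction script runs it to set that starting state.
; Double-clicking runs the parent handler, then passes this actor to OnRight on BP_EventManager, obtained by casting the game mode.
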(fn `OnDoubleClicked`
  (`parent.OnDoubleClicked`)
  (bind _asbp_event_manager (cast `/Game/Blueprints/Event/BP_EventManager` (`GameplayStatics.GetGameMode`)))
  (`/Game/Blueprints/Event/BP_EventManager.OnRight` _asbp_event_manager self))

(fn `Reset`
  (bind _before (`self.before`))
  (`/Engine/EditorBlueprintResources/StandardMacros.IsValid` _before
    (:`Is Valid`
      (`self.SetActorHiddenInGame` _before false)
      (`self.SetActorEnableCollision` _before true))
    (:`Is Not Valid`
      _))
  (`self.SetActorHiddenInGame` true)
  (`self.SetActorEnableCollision` false))

(fn `UserConstructionScript`
  (`parent.UserConstructionScript`)
  (`self.Reset`))
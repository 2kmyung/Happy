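; Event manager that plays a list of events on a shrinking timer, ending in a game-over widget at a fixed index.
; After a right-click starts it, Tick fires the first event immediately, shortens the delay after each event and periodically over time, and quits if the list runs out.
; OnRight and OnWrong chain blink-widget animations through finish delegates: right resets the checked BP_After, wrong adds surprise and sharply cuts the delay.
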(event `Key|RightMouseButton`
  (params (Key :type "Key Structure"))
  (:`Pressed`
    (set `self.isStarted` true)))

(event `self.ReceiveTick`
  (params (DeltaSeconds :type "Float (single-precision)"))
  ;[1 1 1] 대기
  (if (`self.isStarted`)
    (`self.WaitHarder` DeltaSeconds)
    (`self.WaitEvent` DeltaSeconds)))

(event `self.ReceiveBeginPlay`
  (set `self.waitingEvent` (`self.eventDelay`))
  (bind _returnvalue (`|CreateWidget` "/Game/Blueprints/Effects/BP_Blinking.BP_Blinking_C"))
  (set `self.blinking` _returnvalue)
  (`self.EnableInput` (`GameplayStatics.GetPlayerController` 0)))

(fn `DecreaseEventDelay`
  (params (Amount :type "Float (double-precision)"))
  (set `self.eventDelay` (- (`self.eventDelay`) Amount)))

(fn `OnGameOver`
  (bind _returnvalue (`|CreateWidget` "/Game/Blueprints/Widgets/BP_GameOver.BP_GameOver_C"))
  (`UserWidget.AddToViewport` _returnvalue 0)
  (`UserWidget.PlayAnimation` _returnvalue (`/Game/Blueprints/Widgets/BP_GameOver.Show` _returnvalue) 0.0 1 "Forward" 1.0 false))

(fn `OnRight`
  (params (after :type "/Game/Blueprints/Event/BP_After Object Reference"))
  (bind _blinking (`self.blinking`))
  (bind _blinking_2 (`self.blinking`))
  (bind _blinking_3 (`self.blinking`))
  (set `self.checked` after)
  (`UserWidget.AddToViewport` (`self.blinking`) 0)
  (`UserWidget.PlayAnimation` _blinking (`/Game/Blueprints/Effects/BP_Blinking.Close` _blinking) 0.0 1 "Forward" 1.0 false)
  (`UserWidget.BindToAnimationFinished` _blinking_2 (`/Game/Blueprints/Effects/BP_Blinking.Close` _blinking_2) (`|CreateDelegate` :!event `OnRightCloseEnd`))
  (`UserWidget.BindToAnimationFinished` _blinking_3 (`/Game/Blueprints/Effects/BP_Blinking.Open` _blinking_3) (`|CreateDelegate` :!event `OnRightOpenEnd`)))

(fn `OnRightCloseEnd`
  (bind _blinking (`self.blinking`))
  (bind _asbp_after (cast `/Game/Blueprints/Event/BP_After` (`self.checked`)))
  (`/Game/Blueprints/Event/BP_After.Reset` _asbp_after)
  (`UserWidget.PlayAnimation` _blinking (`/Game/Blueprints/Effects/BP_Blinking.Open` _blinking) 0.0 1 "Forward" 1.0 false))

(fn `OnRightOpenEnd`
  (bind _blinking (`self.blinking`))
  (bind _blinking_2 (`self.blinking`))
  (`Widget.RemoveFromParent` (`self.blinking`))
  (`UserWidget.UnbindAllFromAnimationFinished` _blinking (`/Game/Blueprints/Effects/BP_Blinking.Close` _blinking))
  (`UserWidget.UnbindAllFromAnimationFinished` _blinking_2 (`/Game/Blueprints/Effects/BP_Blinking.Open` _blinking_2)))

(fn `OnWrong`
  (params (before :type "/Game/Blueprints/Event/BP_Before Object Reference"))
  (bind _blinking (`self.blinking`))
  (bind _blinking_2 (`self.blinking`))
  (bind _blinking_3 (`self.blinking`))
  (set `self.checked` before)
  (`UserWidget.AddToViewport` (`self.blinking`) 0)
  (`UserWidget.PlayAnimation` _blinking (`/Game/Blueprints/Effects/BP_Blinking.Close` _blinking) 0.0 1 "Forward" 1.0 false)
  (`UserWidget.BindToAnimationFinished` _blinking_2 (`/Game/Blueprints/Effects/BP_Blinking.Close` _blinking_2) (`|CreateDelegate` :!event `OnWrongCloseEnd`))
  (`UserWidget.BindToAnimationFinished` _blinking_3 (`/Game/Blueprints/Effects/BP_Blinking.Surprise` _blinking_3) (`|CreateDelegate` :!event `OnWrongOpenEnd`)))

(fn `OnWrongCloseEnd`
  (bind _blinking (`self.blinking`))
  (`UserWidget.PlayAnimation` _blinking (`/Game/Blueprints/Effects/BP_Blinking.Open` _blinking) 0.0 1 "Forward" 1.0 false)
  (`UserWidget.PlayAnimation` _blinking (`/Game/Blueprints/Effects/BP_Blinking.Surprise` _blinking) 0.0 1 "Forward" 1.0 false)
  (`self.DecreaseEventDelay` 10.0))

(fn `OnWrongOpenEnd`
  (bind _blinking (`self.blinking`))
  (bind _blinking_2 (`self.blinking`))
  (`Widget.RemoveFromParent` (`self.blinking`))
  (`UserWidget.UnbindAllFromAnimationFinished` _blinking (`/Game/Blueprints/Effects/BP_Blinking.Close` _blinking))
  (`UserWidget.UnbindAllFromAnimationFinished` _blinking_2 (`/Game/Blueprints/Effects/BP_Blinking.Surprise` _blinking_2)))

(fn `PlayEvent`
  (if (== (`self.eventIndex`) 3)
    (`self.OnGameOver`)
    (else
      (`/Game/Blueprints/Event/BP_Before.Play` (`|GetArrayItem` (`self.Events`) (`self.eventIndex`)))
      (set `self.eventIndex` (+ (`self.eventIndex`) 1))
      (if (>= (`self.eventIndex`) (`KismetArrayLibrary.Array_Length` (`self.Events`)))
        (`KismetSystemLibrary.QuitGame` null "Quit")))))

(fn `UserConstructionScript`)

(fn `WaitEvent`
  (params (deltaTime :type "Float (double-precision)"))
  (bind _output_get (set `self.waitingEvent` (+ (`self.waitingEvent`) deltaTime)))
  (if (>= _output_get (`self.eventDelay`))
    (`self.PlayEvent`)
    (set `self.waitingEvent` 0.0)
    (set `self.eventDelay` (- (`self.eventDelay`) 1.0))))

(fn `WaitHarder`
  (params (deltaTime :type "Float (double-precision)"))
  (bind _output_get (set `self.waitingHarder` (+ (`self.waitingHarder`) deltaTime)))
  (if (>= _output_get (`self.harderDelay`))
    (`self.DecreaseEventDelay` 0.5)
    (set `self.waitingHarder` 0.0)))